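; BP_HeroCharacter is the player's hero character Blueprint, which sets up the on-screen HUD and a modular soldier head.
; On BeginPlay it creates crosshair, ammo count and health widgets for player controller 0 and adds them to the viewport.
; The construction script makes SoldierHead follow the main Mesh through Leader Pose, so both share one animation pose.
; A key-info widget chain is present but unconnected, and Tick and overlap events are empty.
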(event `self.ReceiveBeginPlay`
  (bind _returnvalue (`GameplayStatics.GetPlayerController` 0))
  (bind _returnvalue_2 (`|CreateWidget` "/Game/Blueprint/Player/Crosshair/WBP_Crosshair.WBP_Crosshair_C" _returnvalue))
  (`UserWidget.AddToViewport` _returnvalue_2 0)
  (bind _returnvalue_3 (`|CreateWidget` "/Game/Blueprint/UI/WB_AmmoCount.WB_AmmoCount_C" _returnvalue))
  (`UserWidget.AddToViewport` _returnvalue_3 0)
  (bind _returnvalue_4 (`|CreateWidget` "/Game/Blueprint/UI/WB_Health.WB_Health_C" _returnvalue))
  (`UserWidget.AddToViewport` _returnvalue_4 0))

(fn `UserConstructionScript`
  (`SkinnedMeshComponent.SetLeaderPoseComponent` (`self.SoldierHead`) (`self.Mesh`) false false))